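; BP_EnemyAI is a Paper2D enemy character that patrols along the X axis and can be damaged and killed.
; While alive, Tick picks an idle or walk flipbook from velocity, faces the sprite along MovementDirection and adds movement input.
; A short forward line trace detects obstacles, and a DoOnce gates the pause before it reverses direction.
; AnyDamage reduces health and applies knockback, showing a hurt flipbook or a death flipbook followed by delayed destruction.
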(event `self.ReceiveBeginPlay`
  (set `CharacterMovementComponent.MaxWalkSpeed` (`self.Max Walk Speed`) (`self.CharacterMovement`)))

(event `self.ReceiveTick`
  (params (DeltaSeconds :type "Float (single-precision)"))
  (if (not (`self.IsDead`))
    (`self.Anim Update`)
    (`self.Movement Update`)))

(event `Anim Update`
  ;[1 1 1] Anim Update
  (`PaperFlipbookComponent.SetFlipbook` (`self.Sprite`) (select `bool` (> (`KismetMathLibrary.VSize` (`MovementComponent.Velocity` (`self.CharacterMovement`))) 0.0) :`false` (`self.FB_Enemy_Idle`) :`true` (`self.FB_Enemy_Walk`))))

(event `Movement Update`
  (bind _returnvalue (`self.K2_GetActorLocation`))
  (bind _charactermovement (`self.CharacterMovement`))
  ;[1 1 1] Movement Update
  (`|ExecutionSequence`
    (:`then_0`
      (if (> (`self.Movement_Direction`) 0.0)
        (`self.K2_SetActorRotation` (struct))
        (else
          (`self.K2_SetActorRotation` (struct :`Yaw` 180.0)))))
    (:`then_1`
      (`self.AddMovementInput` (1.0 0.0 0.0) (`self.Movement_Direction`))
      (bind (_outhit _returnvalue_2) (`KismetSystemLibrary.LineTraceSingle` _returnvalue (+ (* (`self.GetActorForwardVector`) (75.0 0.0 0.0)) _returnvalue) "TraceTypeQuery1"))
      (if _returnvalue_2
        (`/Engine/EditorBlueprintResources/StandardMacros.DoOnce` false :!label _label
          (:`Completed`
            (set `CharacterMovementComponent.MaxWalkSpeed` 0.0 _charactermovement)
            (`KismetSystemLibrary.Delay` (`self.Duration`))
            (set `CharacterMovementComponent.MaxWalkSpeed` (`self.Max Walk Speed`) _charactermovement)
            (set `self.Movement_Direction` (* (`self.Movement_Direction`) -1.0))
            (goto _label :!via `Reset`)))))))

(event `self.ReceiveAnyDamage`
  (params (Damage :type "Float (single-precision)") (DamageType :type "DamageType Object Reference") (InstigatedBy :type "Controller Object Reference") (DamageCauser :type "Actor Object Reference"))
  (bind _returnvalue_x (`KismetMathLibrary.BreakVector` (`KismetMathLibrary.Normal` (`KismetMathLibrary.GetDirectionUnitVector` (`self.K2_GetActorLocation` DamageCauser) (`self.K2_GetActorLocation`)))))
  (set `self.Enemy_Health` (- (`self.Enemy_Health`) Damage))
  (`self.LaunchCharacter` (`KismetMathLibrary.MakeVector` (* (select `bool` (< _returnvalue_x 0.0) :`false` -1.0 :`true` 1.0) -50.0)))
  (if (<= (`self.Enemy_Health`) 0.0)
    (set `self.IsDead` true)
    (`PaperFlipbookComponent.SetFlipbook` (`self.Sprite`) "/Game/ASSets/Textures/Enemies/Puppet64/ded/FB_UndeadExec_Ded.FB_UndeadExec_Ded")
    (`PaperFlipbookComponent.SetLooping` (`self.Sprite`) false)
    (`ActorComponent.K2_DestroyComponent` (`self.CapsuleComponent`))
    (`KismetSystemLibrary.Delay` 2.0)
    (`self.K2_DestroyActor`)
    (else
      (set `self.IsDead` false)
      (`PaperFlipbookComponent.SetFlipbook` (`self.Sprite`) "/Game/ASSets/Textures/Enemies/Puppet64/Hurt/FB_UndeadExec_Hurt.FB_UndeadExec_Hurt")
      (`PaperFlipbookComponent.SetLooping` (`self.Sprite`) false))))

(fn `UserConstructionScript`)